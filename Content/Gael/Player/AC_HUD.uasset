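; AC_HUD is a player component that puts the HUD on screen and starts the player character's timer in every level except Main_Menu.
; On BeginPlay it checks the level name, creates a W_Hud widget for the first player controller, stores the reference and adds it to the viewport.
; It then casts the player pawn to BP_ThirdPersonCharacter and calls its Timer function.
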(event Custom|StartTimer
  (bind _asbp_third_person_character (Utilities|Casting|CastToBP_ThirdPersonCharacter (Game|Player|GetPlayerPawn 0)))
  (Default|Timer _asbp_third_person_character))

(event EventBeginPlay
  (bind _returnvalue (Game|GetCurrentLevelName true))
  (if (Utilities|Enum|NotEqual(Enum) _returnvalue "Main_Menu")
    (bind _returnvalue_2 (UserInterface|CreateWidget "/Game/Gael/Player/W_Hud.W_Hud_C" (Game|GetPlayerController 0)))
    (Variables|Default|SethudWidgetRef _returnvalue_2)
    (UserInterface|Viewport|AddtoViewport _returnvalue_2 0)
    (CallFunction|StartTimer)))