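; BP_VillagerBase is a base villager that the player can target and that removes itself after death.
; Overlapping its sphere sets or clears it as the third-person character's Target and toggles the WAttack widget.
; Tick rotates that widget to face the player's follow camera.
; Death clears IsAlive, which makes the show/hide event hide the widget, then destroys the actor after a short delay.
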(event OnComponentBeginOverlap(Sphere)
  (params (OverlappedComponent :type Primitive%20Component%20Object%20Reference) (OtherActor :type Actor%20Object%20Reference) (OtherComp :type Primitive%20Component%20Object%20Reference) (OtherBodyIndex :type Integer) (bFromSweep :type Boolean) (SweepResult :type Hit%20Result%20Structure%20%28by%20ref%29))
  (bind _asbp_third_person_character (Utilities|Casting|CastToBP_ThirdPersonCharacter OtherActor))
  (Variables|/Game/ThirdPerson/Blueprints/BP_ThirdPersonCharacter.BP_ThirdPersonCharacter_C|Settarget _asbp_third_person_character self)
  (CallFunction|Show/HideWidget))

(event OnComponentEndOverlap(Sphere)
  (params (OverlappedComponent :type Primitive%20Component%20Object%20Reference) (OtherActor :type Actor%20Object%20Reference) (OtherComp :type Primitive%20Component%20Object%20Reference) (OtherBodyIndex :type Integer))
  (bind _asbp_third_person_character (Utilities|Casting|CastToBP_ThirdPersonCharacter OtherActor))
  (Variables|/Game/ThirdPerson/Blueprints/BP_ThirdPersonCharacter.BP_ThirdPersonCharacter_C|Settarget _asbp_third_person_character 0)
  (CallFunction|Show/HideWidget))

(event Custom|Show/Hide%20Widget
  (if (Variables|Default|GetisAlive?)
    (Rendering|ToggleVisibility (Variables|Default|GetW_Attack) false)
    (else
      (Rendering|SetVisibility (Variables|Default|GetW_Attack) false false))))

(event Custom|Death
  (Variables|Default|SetisAlive? false)
  (CallFunction|Show/HideWidget)
  (Utilities|FlowControl|Delay 3.0)
  (Actor|DestroyActor))

(event EventTick
  (params (DeltaSeconds :type Float%20%28single-precision%29))
  (bind _asbp_third_person_character (Utilities|Casting|CastToBP_ThirdPersonCharacter (Game|Player|GetPlayerPawn 0)))
  (Transformation|SetWorldRotation (Variables|Default|GetW_Attack) (Math|Rotator|FindLookatRotation (Transformation|GetWorldLocation (Variables|Default|GetW_Attack)) (Transformation|GetWorldLocation (Variables|/Game/ThirdPerson/Blueprints/BP_ThirdPersonCharacter.BP_ThirdPersonCharacter_C|GetFollowCamera _asbp_third_person_character))) false false))

(fn ConstructionScript)