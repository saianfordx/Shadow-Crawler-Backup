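; BP_EndDetector is an end-of-level detector actor that shows the End_Game_Menu widget when the player character comes near it.
; Every Tick, DetectPlayer runs a stationary multi-sphere trace around the actor, with debug drawing enabled.
; Each hit that casts to BP_ThirdPersonCharacter calls OpenWinMenu, which creates the menu and adds it to the viewport.
; No guard prevents repeated menu creation while the player stays in range.
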(event EventBeginPlay)

(event Collision|EventActorBeginOverlap
  (params (OtherActor :type Actor%20Object%20Reference)))

(event EventTick
  (params (DeltaSeconds :type Float%20%28single-precision%29))
  (CallFunction|DetectPlayer))

(fn ConstructionScript)

(fn DetectPlayer
  (bind _outhits (Collision|MultiSphereTraceByChannel (Transformation|GetActorLocation) (Transformation|GetActorLocation) 2e+02 "TraceTypeQuery3" false 0 "ForDuration"))
  (for _array_element _outhits
    (Utilities|Casting|CastToBP_ThirdPersonCharacter (.HitActor (Collision|BreakHitResult _array_element)))
    (CallFunction|OpenWinMenu)))

(fn OpenWinMenu
  (bind _returnvalue (UserInterface|CreateWidget "/Game/Source/Widgets/End_Game_Menu.End_Game_Menu_C" (Game|GetPlayerController 0)))
  (UserInterface|Viewport|AddtoViewport _returnvalue 0))