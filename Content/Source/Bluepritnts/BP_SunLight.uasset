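; BP_SunLight is a sun actor that damages the player while they are exposed to it during the day.
; Every tick, TracePlayer finds BP_EnvTool and checks IsDay, then line traces from its own location to the player's capsule.
; If the trace hits BP_ThirdPersonCharacter, it applies DPS to that character's CPHealth, once per tick without delta-time scaling.
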(event EventTick
  (params (DeltaSeconds :type Float%20%28single-precision%29))
  ;[1 1 1] Find Player - If Day Light and Makes Damage IIf Finds Him
  (CallFunction|TracePlayer))

(fn ConstructionScript)

(fn TracePlayer
  (bind _returnvalue (Actor|GetActorOfClass "/Game/Source/Bluepritnts/BP_EnvTool.BP_EnvTool_C"))
  (if (Variables|/Game/Source/Bluepritnts/BP_EnvTool.BP_EnvTool_C|GetIsDay _returnvalue)
    (bind _outhit (Collision|LineTraceByChannel (Transformation|GetActorLocation) (Transformation|GetWorldLocation (Variables|/Script/Engine.Character|GetCapsuleComponent (Game|GetPlayerCharacter 0))) "TraceTypeQuery3" false 0 "None"))
    (bind _asbp_third_person_character (Utilities|Casting|CastToBP_ThirdPersonCharacter (.HitActor (Collision|BreakHitResult _outhit))))
    (Default|ApplyDamage (Variables|/Game/ThirdPerson/Blueprints/BP_ThirdPersonCharacter.BP_ThirdPersonCharacter_C|GetCP_Health _asbp_third_person_character) (Variables|Default|GetDPS))))