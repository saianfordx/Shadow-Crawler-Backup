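; BP_SunLightCapsule is a moving sunlight hazard that damages the third-person player character within a large radius.
; On BeginPlay, it reads IsDay from BP_EnvTool and, if true, slides its root to EndGameLocation over a fixed time.
; Every Tick, DetectPlayer runs a sphere trace at its location with persistent debug drawing, applying damage through the character's CPHealth regardless of IsDay.
; TranportToEnd is an empty stub.
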(event EventBeginPlay
  (bind _returnvalue (Actor|GetActorOfClass "/Game/Source/Bluepritnts/BP_EnvTool.BP_EnvTool_C"))
  (if (Variables|/Game/Source/Bluepritnts/BP_EnvTool.BP_EnvTool_C|GetIsDay _returnvalue)
    (Components|MoveComponentTo (Variables|Default|GetDefaultSceneRoot) (Variables|Default|GetEnd%20Game%20Location) "0, 0, 0" false false 1e+01 false)))

(event EventTick
  (params (DeltaSeconds :type Float%20%28single-precision%29))
  (CallFunction|DetectPlayer))

(fn ConstructionScript)

(fn DetectPlayer
  (bind _outhits (Collision|MultiSphereTraceByChannel (Transformation|GetActorLocation) (Transformation|GetActorLocation) 2.5e+03 "TraceTypeQuery3" false 0 "Persistent"))
  (for _array_element _outhits
    (bind _asbp_third_person_character (Utilities|Casting|CastToBP_ThirdPersonCharacter (.HitActor (Collision|BreakHitResult _array_element))))
    (Default|ApplyDamage (Variables|/Game/ThirdPerson/Blueprints/BP_ThirdPersonCharacter.BP_ThirdPersonCharacter_C|GetCP_Health _asbp_third_person_character) 0.5)))

(fn TranporttoEnd
  (params (DeltaTime :type Float%20%28double-precision%29)))